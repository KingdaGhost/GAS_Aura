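; Flame pillar actor that flickers its fire light continuously from BeginPlay.
; It randomly picks one of two intensity timelines, then picks again whenever the current one finishes, so the flicker pattern varies.
; Each timeline update feeds SetLightIntensity, which scales the curve value by the LightIntensity variable and applies it to FireLight.
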(event `self.ReceiveBeginPlay`
  (`self.ChooseTimeline`))

(event `ChooseTimeline`
  (switch `int` (`KismetMathLibrary.RandomIntegerInRange` 0 1)
    (:`Default`
      (`self.PlayFireIntensity_2` :!label _label))
    (:`0`
      (`self.PlayFireIntensity_1`))
    (:`1`
      (goto _label))))

(event `PlayFireIntensity_1`
  (bind (_direction _lightintensity) (`Timeline|FireIntesity_1` :!via `PlayFromStart`)
    (:`Update`
      (`self.SetLightIntensity` _lightintensity))
    (:`Finished`
      (`self.ChooseTimeline`))))

(event `PlayFireIntensity_2`
  (bind (_direction _lightintensity) (`Timeline|FireIntensity_2` :!via `PlayFromStart`)
    (:`Update`
      (`self.SetLightIntensity` _lightintensity))
    (:`Finished`
      (`self.ChooseTimeline`))))

(fn `SetLightIntensity`
  (params (Intensity :type "Float (double-precision)"))
  (`LightComponent.SetIntensity` (`self.FireLight`) (* Intensity (`self.LightIntensity`))))

(fn `UserConstructionScript`)