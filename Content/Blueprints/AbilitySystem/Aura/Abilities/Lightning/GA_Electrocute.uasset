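; GA_Electrocute is a lightning ability that channels an electric beam from the owner's weapon toward the mouse target until input is released.
; Activation stores mouse target data, faces the target and plays a montage, whose gameplay event locks movement and starts the beam.
; The looping ShockLoop cue attaches to combat targets, otherwise to the avatar; release removes it and restores movement and cursor.
; Additional targets are gathered but not yet processed.
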(event `self.K2_ActivateAbility`
  (`self.EnforceImplementsCombatInterface`)
  ;[0.1556 0.142 1] Store Mouse Data Variables
  (bind (_asynctaskproxy _datahandle) (`TargetDataUnderMouse.CreateTargetDataUnderMouse`)
    (:`ValidData`
      (`self.StoreMouseDataInfo` (`AbilitySystemBlueprintLibrary.GetHitResultFromTargetData` _datahandle))
      (`self.StoreOwnerVariables`)
      (`|ExecutionSequence`
        (:`then_0`
          (set `PlayerController.bShowMouseCursor` false (`self.OwnerPlayerController`))
          (`self.UpdateFacingTarget`)
          ;[1 1 1] Play Sound
          (`self.K2_ExecuteGameplayCue` (struct :`TagName` "GameplayCue.ShockBurst"))
          (`AbilityTask_PlayMontageAndWait.CreatePlayMontageAndWaitProxy` "None" (`self.Montage_Electrocute`)
            (:`then`
              ;[0 0.3125 0.2885 1 15] This is for Motion Warping. Motion Warping happens before we send out this Event Tag
              (`AbilityTask_WaitGameplayEvent.WaitGameplayEvent` (struct :`TagName` "Event.Montage.Electrocute") null
                (:`EventReceived`
                  (`self.InShockLoop`)
                  (`self.SpawnElectricBeam`))))))
        (:`then_1`
          (`AbilityTask_WaitInputRelease.WaitInputRelease` false
            (:`OnRelease`
              (`self.PrepareToEndAbility`)
              (`self.K2_EndAbility`))))))))

(fn `EnforceImplementsCombatInterface`
  (if (not (`KismetSystemLibrary.DoesImplementInterface` (`self.GetAvatarActorFromActorInfo`) "/Script/Aura.CombatInterface"))
    (`self.K2_EndAbility`)))

(fn `InShockLoop`
  (message `CombatInterface.SetInShockLoop` (`self.OwnerCharacter`) true)
  (`CharacterMovementComponent.DisableMovement` (`Character.CharacterMovement` (`self.OwnerCharacter`))))

(fn `PrepareToEndAbility`
  (set `PlayerController.bShowMouseCursor` true (`self.OwnerPlayerController`))
  (message `CombatInterface.SetInShockLoop` (`self.OwnerCharacter`) false)
  (`CharacterMovementComponent.SetMovementMode` (`Character.CharacterMovement` (`self.OwnerCharacter`)) "MOVE_Walking" 0)
  (if (`self.bFirstTargetImplemetsInterface`)
    (`GameplayCueFunctionLibrary.RemoveGameplayCueOnActor` (`self.MouseHitActor`) (struct :`TagName` "GameplayCue.ShockLoop") (`self.FirstTargetCueParams`))
    (else
      (`GameplayCueFunctionLibrary.RemoveGameplayCueOnActor` (`self.GetAvatarActorFromActorInfo`) (struct :`TagName` "GameplayCue.ShockLoop") (`self.FirstTargetCueParams`)))))

(fn `SpawnElectricBeam`
  (locals (CueTarget :type "Actor Object Reference"))
  (`self.TraceFirstTarget` (`self.MouseHitLocation`))
  (bind _returnvalue (message `CombatInterface.GetWeapon` (`self.OwnerCharacter`)))
  (set `self.FirstTargetCueParams` (`AbilitySystemBlueprintLibrary.MakeGameplayCueParameters` 0.0 0.0 (struct) (struct) (struct) (struct) (struct) (`self.MouseHitLocation`) (0.0 0.0 0.0) null null (`self.MouseHitActor`) null 1 1 _returnvalue))
  ;[1 1 1] Is MouseHitActor an Enemy?
  (bind _output_get (set `self.bFirstTargetImplemetsInterface` (`KismetSystemLibrary.DoesImplementInterface` (`self.MouseHitActor`) "/Script/Aura.CombatInterface")))
  (if _output_get
    (set `local.CueTarget` (`self.MouseHitActor`))
    (else
      (set `local.CueTarget` (`self.GetAvatarActorFromActorInfo`))))
  (`GameplayCueFunctionLibrary.AddGameplayCueOnActor` (`local.CueTarget`) (struct :`TagName` "GameplayCue.ShockLoop") (`self.FirstTargetCueParams`))
  (bind _outadditionaltargets (`self.StoreAdditionalTargets`))
  (for _ _outadditionaltargets
    _))

(fn `UpdateFacingTarget`
  (message `CombatInterface.UpdateFacingTarget` (`self.OwnerCharacter`) (`self.MouseHitLocation`)))