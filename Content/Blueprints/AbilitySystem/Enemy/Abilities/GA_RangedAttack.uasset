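; Enemy gameplay ability that fires a projectile at the avatar's current combat target.
; On activation it turns the avatar toward the target through CombatInterface and plays a random tagged attack montage.
; A gameplay event matching the montage's tag triggers SpawnProjectile toward the target location captured at activation, then ends the ability.
; The ability also ends if the montage completes, is interrupted or is cancelled.
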(event `self.K2_ActivateAbility`
  (bind _returnvalue (`self.GetAvatarActorFromActorInfo`))
  (bind _returnvalue_2 (message `EnemyInterface.GetCombatTarget` _returnvalue))
  (set `self.TargetLocation` (`Actor.K2_GetActorLocation` _returnvalue_2))
  (bind _ascombat_interface (cast `CombatInterface` _returnvalue))
  (`CombatInterface.UpdateFacingTarget` _ascombat_interface (`self.TargetLocation`))
  (bind _output_get (set `self.TaggedMontage` (`self.GetRandomTaggedMontageFromArray` (`CombatInterface.GetAttackMontages` _ascombat_interface))))
  (bind (_montage _montagetag) (break `TaggedMontage` _output_get))
  (`AbilityTask_PlayMontageAndWait.CreatePlayMontageAndWaitProxy` "None" _montage 1.0 "None" false
    (:`then`
      (`AbilityTask_WaitGameplayEvent.WaitGameplayEvent` _montagetag null
        (:`EventReceived`
          (message `CombatInterface.GetCombatSocketLocation` (`self.GetAvatarActorFromActorInfo`) _montagetag)
          (`self.SpawnProjectile` (`self.TargetLocation`))
          (`self.K2_EndAbility`))))
    (:`OnCompleted`
      (`self.K2_EndAbility` :!label _label))
    (:`OnInterrupted`
      (goto _label))
    (:`OnCancelled`
      (goto _label))))